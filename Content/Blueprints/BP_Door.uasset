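; BP_Door is an interactable door that swings open or closed when a character interacts with it, unless it is locked.
; Interact plays an opening animation on the character's mesh, waits briefly, then returns the mesh to its Animation Blueprint.
; It toggles IsOpen and plays or reverses a rotation timeline that drives the DoorPack's yaw.
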(event `self.Interact`
  (params (Character :type "/Game/ThirdPerson/Blueprints/BP_ThirdPersonCharacter Object Reference"))
  (bind _mesh (`Character.Mesh` Character))
  (bind _mesh_2 (`Character.Mesh` Character))
  (if (`self.Locked`)
    _
    (elif (not (`self.IsOpen`))
      (`SkeletalMeshComponent.PlayAnimation` _mesh "/Game/ThirdPerson/Blueprints/Opening.Opening" false)
      (`KismetSystemLibrary.Delay` 0.5)
      (`SkeletalMeshComponent.SetAnimationMode` _mesh "AnimationBlueprint" true)
      (set `self.IsOpen` true)
      (bind (_direction _newtrack_0) (`Timeline|DoorRotationTimeline` :!label _label)
        (:`Update`
          (`SceneComponent.K2_SetRelativeRotation` (`self.DoorPack`) (`KismetMathLibrary.MakeRotator` 0.0 0.0 _newtrack_0) false false)))
      (else
        (`SkeletalMeshComponent.PlayAnimation` _mesh_2 "/Game/ThirdPerson/Blueprints/Opening.Opening" false)
        (`KismetSystemLibrary.Delay` 0.5)
        (`SkeletalMeshComponent.SetAnimationMode` _mesh_2 "AnimationBlueprint" true)
        (set `self.IsOpen` false)
        (goto _label :!via `Reverse`)))))

(fn `UserConstructionScript`)