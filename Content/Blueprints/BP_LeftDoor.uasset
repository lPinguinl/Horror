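; BP_LeftDoor is an interactable door Blueprint that swings open and closed unless it is Locked.
; Interact toggles IsOpen and plays or reverses a timeline that drives the yaw of DoorPack's relative rotation.
; During timeline updates, a 2D Scary_Door sound is spawned and faded in whenever the stored OpenCloseDoor audio component is not valid.
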(event `self.Interact`
  (if (`self.Locked`)
    _
    (elif (not (`self.IsOpen`))
      (set `self.IsOpen` true)
      (bind (_direction _newtrack_0) (`Timeline|DoorRotationTimeline` :!label _label)
        (:`Update`
          (`SceneComponent.K2_SetRelativeRotation` (`self.DoorPack`) (`KismetMathLibrary.MakeRotator` 0.0 0.0 _newtrack_0) false false)
          (`self.Open_Close_Door`
            (:`then`)
            (:`else`
              (bind _returnvalue (`GameplayStatics.SpawnSound2D` "/Game/Audio/Scary_Door.Scary_Door" 1.0 1.0 0.0 null))
              (bind _output_get (set `self.Open_Close_Door` _returnvalue))
              (`AudioComponent.FadeIn` _output_get 0.2 1.0 0.0 "Linear")))))
      (else
        (set `self.IsOpen` false)
        (goto _label :!via `Reverse`)))))

(fn `UserConstructionScript`)