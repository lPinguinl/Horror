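; BP_LeftDoorTuto is an interactable tutorial door that swings open and closed unless it is locked.
; Interact toggles IsOpen and plays or reverses a timeline that drives the yaw of DoorPack.
; Timeline updates spawn and fade in a 2D creak sound whenever no valid sound reference exists.
; A trigger overlap shows the widget while the third-person character is in range and hides it on exit.
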(event `self.Interact`
  (if (`self.Locked`)
    _
    (elif (not (`self.IsOpen`))
      (set `self.IsOpen` true)
      (bind (_direction _newtrack_0) (`Timeline|DoorRotationTimeline` :!label _label)
        (:`Update`
          (`SceneComponent.K2_SetRelativeRotation` (`self.DoorPack`) (`KismetMathLibrary.MakeRotator` 0.0 0.0 _newtrack_0) false false)
          (`self.Open_Close_Door`
            (:`then`)
            (:`else`
              (bind _returnvalue (`GameplayStatics.SpawnSound2D` "/Game/Audio/Scary_Door.Scary_Door" 1.0 1.0 0.0 null))
              (bind _output_get (set `self.Open_Close_Door` _returnvalue))
              (`AudioComponent.FadeIn` _output_get 0.2 1.0 0.0 "Linear")))))
      (else
        (set `self.IsOpen` false)
        (goto _label :!via `Reverse`)))))

(event `self.Trigger.OnComponentBeginOverlap`
  (params (OverlappedComponent :type "PrimitiveComponent Object Reference") (OtherActor :type "Actor Object Reference") (OtherComp :type "PrimitiveComponent Object Reference") (OtherBodyIndex :type Integer) (bFromSweep :type Boolean) (SweepResult :type "HitResult Structure (by ref)"))
  (cast `/Game/ThirdPerson/Blueprints/BP_ThirdPersonCharacter` OtherActor)
  (`SceneComponent.SetVisibility` (`self.Widget`) true false))

(event `self.Trigger.OnComponentEndOverlap`
  (params (OverlappedComponent :type "PrimitiveComponent Object Reference") (OtherActor :type "Actor Object Reference") (OtherComp :type "PrimitiveComponent Object Reference") (OtherBodyIndex :type Integer))
  (cast `/Game/ThirdPerson/Blueprints/BP_ThirdPersonCharacter` OtherActor)
  (`SceneComponent.SetVisibility` (`self.Widget`) false false))

(fn `UserConstructionScript`)