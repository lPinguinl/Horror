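; Tutorial drawer that the player can get into and out of by interacting with it.
; Interact toggles InsideDrawer and teleports player character 0 to the location and rotation of the REFInside or REFOutside marker.
; A single timeline drives the yaw of DoorPack, running in reverse on entry and forward on exit.
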(event `self.Interact`
  (bind (_returnvalue_location _returnvalue_rotation) (`KismetMathLibrary.BreakTransform` (`SceneComponent.K2_GetComponentToWorld` (`self.REF Inside`))))
  (bind (_returnvalue_location_2 _returnvalue_rotation_2) (`KismetMathLibrary.BreakTransform` (`SceneComponent.K2_GetComponentToWorld` (`self.REF Outside`))))
  (if (not (`self.insideDrawer`))
    (set `self.insideDrawer` true)
    (`self.K2_SetActorTransform` (`GameplayStatics.GetPlayerCharacter` 0) (`KismetMathLibrary.MakeTransform` _returnvalue_location _returnvalue_rotation) false false)
    (bind (_direction _newtrack_0) (`Timeline|Timeline` :!via `Reverse` :!label _label)
      (:`Update`
        (`SceneComponent.K2_SetRelativeRotation` (`self.DoorPack`) (`KismetMathLibrary.MakeRotator` 0.0 0.0 _newtrack_0) false false)))
    (else
      (set `self.insideDrawer` false)
      (`self.K2_SetActorTransform` (`GameplayStatics.GetPlayerCharacter` 0) (`KismetMathLibrary.MakeTransform` _returnvalue_location_2 _returnvalue_rotation_2) false false)
      (goto _label))))

(fn `UserConstructionScript`)