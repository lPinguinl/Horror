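; BP_DoorLoockedLvl1 is a lockable door that swings open or closed when interacted with.
; The Interact event does nothing while Locked is set, and nothing in this graph changes that flag.
; Otherwise it flips IsOpen and runs a Timeline that drives the relative yaw of DoorPack.
; The Timeline runs in reverse when IsOpen becomes true and forward when it becomes false.
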(event `self.Interact`
  (if (`self.Locked`)
    _
    (elif (not (`self.IsOpen`))
      (set `self.IsOpen` true)
      (bind (_direction _newtrack_0) (`Timeline|Timeline` :!via `Reverse` :!label _label)
        (:`Update`
          (`SceneComponent.K2_SetRelativeRotation` (`self.DoorPack`) (`KismetMathLibrary.MakeRotator` 0.0 0.0 _newtrack_0) false false)))
      (else
        (set `self.IsOpen` false)
        (goto _label)))))

(fn `UserConstructionScript`)